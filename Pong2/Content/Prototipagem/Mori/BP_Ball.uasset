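; Physics-driven ball actor that launches along X at BeginPlay and bounces off PlayerBarra paddles, apparently for a Pong-style prototype.
; ResetBall stops it, teleports the sphere to its relative origin, then relaunches it after two seconds in the given direction.
; Tick tracks velocity as |X|+|Y|; paddle hits wait through three zero-length delays, then restore Speed along the 2D heading if that value dropped below it.
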(event OnComponentHit(Sphere)
  (params (HitComponent :type Primitive%20Component%20Object%20Reference) (OtherActor :type Actor%20Object%20Reference) (OtherComp :type Primitive%20Component%20Object%20Reference) (NormalImpulse :type Vector :default "0, 0, 0") (Hit :type Hit%20Result%20Structure%20%28by%20ref%29))
  (Utilities|Casting|CastToPlayerBarra OtherActor)
  (Utilities|FlowControl|Delay 0.0)
  (Utilities|FlowControl|Delay 0.0)
  (Utilities|FlowControl|Delay 0.0)
  (if (< (Variables|Default|GetBallVelocity) (Variables|Default|GetSpeed))
    (CallFunction|SetVelocityasSpeed)))

(event Custom|ResetBall
  (params (direc :type Integer))
  (bind _sphere (Variables|Default|GetSphere))
  (Physics|SetPhysicsLinearVelocity _sphere "0, 0, 0" false "None")
  (Transformation|SetRelativeLocation _sphere "0, 0, 0" false true)
  (Utilities|FlowControl|Delay 2.0)
  (Physics|AddImpulse _sphere (Math|Vector|MakeVector (* direc (Variables|Default|GetSpeed)) 0.0 0.0) "None" true))

(event EventBeginPlay
  (Physics|AddImpulse (Variables|Default|GetSphere) (Math|Vector|MakeVector (Variables|Default|GetSpeed) 0.0 0.0) "None" true))

(event Collision|EventActorBeginOverlap
  (params (OtherActor :type Actor%20Object%20Reference)))

(event EventTick
  (params (DeltaSeconds :type Float%20%28single-precision%29))
  (bind _sphere (Variables|Default|GetSphere))
  (bind _returnvalue (Transformation|GetComponentVelocity _sphere))
  (bind (_x _y) (Math|Vector|BreakVector _returnvalue))
  (Variables|Default|SetBallVelocity (+ (Math|Float|Absolute(Float) _x) (Math|Float|Absolute(Float) _y))))

(fn ConstructionScript)

(fn SetVelocityasSpeed
  (bind _sphere (Variables|Default|GetSphere))
  (Physics|SetPhysicsLinearVelocity _sphere (* (Class|KismetMathLibrary|VectorNormal2D (Transformation|GetComponentVelocity _sphere) 0.0) (Variables|Default|GetSpeed)) false "None"))

(fn SetSpeedasVelocity
  (Variables|Default|SetSpeed (Variables|Default|GetBallVelocity)))