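; Prototype test field Blueprint with a goal area for each of the two players, where ball hits cost that player HP.
; Each area's component hit event reacts only to BP_Ball, finds NewControllerGame_BP via GetActorOfClass, deducts one HP from the matching player's data and refreshes the HUD.
; It then calls ResetBall on the ball, passing the same argument for both goals.
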(event OnComponentHit(AreaGolPlayer1)
  (params (HitComponent :type Primitive%20Component%20Object%20Reference) (OtherActor :type Actor%20Object%20Reference) (OtherComp :type Primitive%20Component%20Object%20Reference) (NormalImpulse :type Vector :default "0, 0, 0") (Hit :type Hit%20Result%20Structure%20%28by%20ref%29))
  (bind _asbp_ball (Utilities|Casting|CastToBP_Ball OtherActor))
  (Utilities|FlowControl|Sequence
    (:then_0
      (bind _returnvalue (Actor|GetActorOfClass "/Game/Prototipagem/Mori/NewControllerGame_BP.NewControllerGame_BP_C"))
      (Default|ModifyHPOfPlayer _returnvalue (Variables|/Game/Prototipagem/Mori/NewControllerGame_BP.NewControllerGame_BP_C|GetP1Data _returnvalue) -1)
      (Default|ApplyHPtoHUD _returnvalue (Variables|/Game/Prototipagem/Mori/NewControllerGame_BP.NewControllerGame_BP_C|GetP1Data _returnvalue)))
    (:then_1
      (Default|ResetBall _asbp_ball 1))))

(event OnComponentHit(AreaGolPlayer2)
  (params (HitComponent :type Primitive%20Component%20Object%20Reference) (OtherActor :type Actor%20Object%20Reference) (OtherComp :type Primitive%20Component%20Object%20Reference) (NormalImpulse :type Vector :default "0, 0, 0") (Hit :type Hit%20Result%20Structure%20%28by%20ref%29))
  (bind _asbp_ball (Utilities|Casting|CastToBP_Ball OtherActor))
  (Utilities|FlowControl|Sequence
    (:then_0
      (bind _returnvalue (Actor|GetActorOfClass "/Game/Prototipagem/Mori/NewControllerGame_BP.NewControllerGame_BP_C"))
      (Default|ModifyHPOfPlayer _returnvalue (Variables|/Game/Prototipagem/Mori/NewControllerGame_BP.NewControllerGame_BP_C|GetP2Data _returnvalue) -1)
      (Default|ApplyHPtoHUD _returnvalue (Variables|/Game/Prototipagem/Mori/NewControllerGame_BP.NewControllerGame_BP_C|GetP2Data _returnvalue)))
    (:then_1
      (Default|ResetBall _asbp_ball 1))))

(event EventBeginPlay)

(event Collision|EventActorBeginOverlap
  (params (OtherActor :type Actor%20Object%20Reference)))

(event EventTick
  (params (DeltaSeconds :type Float%20%28single-precision%29)))

(fn ConstructionScript)