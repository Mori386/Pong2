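; Prototype boss-fight actor with three ball-breakable weak points and hazards that debuff the player's PlayerBarra.
; An endless BeginPlay loop slides the Ataque component to a target, teleports it back and pauses before repeating.
; Each weak-point sphere has its own hit counter, reduced by BP_Ball hits, and is destroyed when depleted.
; Three cube overlaps share one ApplyDebuff call wired to all three PlayerBarra cast results.
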(event OnComponentHit(Sphere)
  (params (HitComponent :type Primitive%20Component%20Object%20Reference) (OtherActor :type Actor%20Object%20Reference) (OtherComp :type Primitive%20Component%20Object%20Reference) (NormalImpulse :type Vector :default "0, 0, 0") (Hit :type Hit%20Result%20Structure%20%28by%20ref%29))
  (Utilities|Casting|CastToBP_Ball OtherActor)
  (if (<= (- (Variables|Default|GetHPWeakPoint) 1) 0)
    (Components|DestroyComponent HitComponent)
    (else
      (Variables|Default|SetHPWeakPoint (- (Variables|Default|GetHPWeakPoint) 1)))))

(event OnComponentHit(Sphere1)
  (params (HitComponent :type Primitive%20Component%20Object%20Reference) (OtherActor :type Actor%20Object%20Reference) (OtherComp :type Primitive%20Component%20Object%20Reference) (NormalImpulse :type Vector :default "0, 0, 0") (Hit :type Hit%20Result%20Structure%20%28by%20ref%29))
  (Utilities|Casting|CastToBP_Ball OtherActor)
  (if (<= (- (Variables|Default|GetHPWeakPoint_0) 1) 0)
    (Components|DestroyComponent HitComponent)
    (else
      (Variables|Default|SetHPWeakPoint_0 (- (Variables|Default|GetHPWeakPoint_0) 1)))))

(event OnComponentHit(Sphere2)
  (params (HitComponent :type Primitive%20Component%20Object%20Reference) (OtherActor :type Actor%20Object%20Reference) (OtherComp :type Primitive%20Component%20Object%20Reference) (NormalImpulse :type Vector :default "0, 0, 0") (Hit :type Hit%20Result%20Structure%20%28by%20ref%29))
  (Utilities|Casting|CastToBP_Ball OtherActor)
  (if (<= (- (Variables|Default|GetHPWeakPoint_1) 1) 0)
    (Components|DestroyComponent HitComponent)
    (else
      (Variables|Default|SetHPWeakPoint_1 (- (Variables|Default|GetHPWeakPoint_1) 1)))))

(event OnComponentBeginOverlap(Cube1)
  (params (OverlappedComponent :type Primitive%20Component%20Object%20Reference) (OtherActor :type Actor%20Object%20Reference) (OtherComp :type Primitive%20Component%20Object%20Reference) (OtherBodyIndex :type Integer) (bFromSweep :type Boolean) (SweepResult :type Hit%20Result%20Structure%20%28by%20ref%29))
  (bind _asplayer_barra (Utilities|Casting|CastToPlayerBarra OtherActor))
  (Default|ApplyDebuff _asplayer_barra))

(event OnComponentBeginOverlap(Cube2)
  (params (OverlappedComponent :type Primitive%20Component%20Object%20Reference) (OtherActor :type Actor%20Object%20Reference) (OtherComp :type Primitive%20Component%20Object%20Reference) (OtherBodyIndex :type Integer) (bFromSweep :type Boolean) (SweepResult :type Hit%20Result%20Structure%20%28by%20ref%29))
  (bind _asplayer_barra (Utilities|Casting|CastToPlayerBarra OtherActor))
  (Default|ApplyDebuff (stale OnComponentBeginOverlap(Cube1) _asplayer_barra)))

(event OnComponentBeginOverlap(Cube3)
  (params (OverlappedComponent :type Primitive%20Component%20Object%20Reference) (OtherActor :type Actor%20Object%20Reference) (OtherComp :type Primitive%20Component%20Object%20Reference) (OtherBodyIndex :type Integer) (bFromSweep :type Boolean) (SweepResult :type Hit%20Result%20Structure%20%28by%20ref%29))
  (bind _asplayer_barra (Utilities|Casting|CastToPlayerBarra OtherActor))
  (Default|ApplyDebuff (stale OnComponentBeginOverlap(Cube1) _asplayer_barra)))

(event EventBeginPlay
  (bind _ataque (Variables|Default|GetAtaque))
  (Components|MoveComponentTo _ataque "-180.000000, 0, 0" "0, 0, 0" false false 5.0 false :!label _label)
  (Transformation|SetWorldLocation _ataque "-105.000000,0.000000,7.000000" false true)
  (Utilities|FlowControl|Delay 2.0)
  (goto _label))

(event Collision|EventActorBeginOverlap
  (params (OtherActor :type Actor%20Object%20Reference)))

(event EventTick
  (params (DeltaSeconds :type Float%20%28single-precision%29)))

(fn ConstructionScript)