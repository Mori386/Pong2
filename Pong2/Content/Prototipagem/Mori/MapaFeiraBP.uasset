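; MapaFeiraBP is a map actor that periodically targets one of the two players with a thrown-item marker, which may be a buff.
; BeginPlay runs an endless delay loop that calls Fire every few seconds.
; Fire randomly picks a player from ControllerGame and spawns an AlvoItemJogado at their location with random Y jitter.
; It assigns that player as the aimed target and turns the item into a buff half the time.
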(event Custom|Fire
  (bind _returnvalue (Actor|GetActorOfClass "/Game/Prototipagem/Mori/ControllerGame.ControllerGame_C"))
  ;[1 0.09375 0.09375] Selecionar o player
  (switch int (Math|Random|RandomIntegerinRange 1 2)
    (:1
      (bind _returnvalue_2 (Game|SpawnActorfromClass "/Game/Prototipagem/Mori/AlvoItemJogado.AlvoItemJogado_C" (Math|Conversions|ToTransform(Vector) (Math|Vector|MakeVector (.X (Math|Vector|BreakVector (Transformation|GetActorLocation (Variables|/Game/Prototipagem/Mori/ControllerGame.ControllerGame_C|GetPlayer1 _returnvalue)))) (+ (.Y (Math|Vector|BreakVector (Transformation|GetActorLocation (Variables|/Game/Prototipagem/Mori/ControllerGame.ControllerGame_C|GetPlayer1 _returnvalue)))) (Math|Random|RandomFloatinRange -3e+01 3e+01)) (.Z (Math|Vector|BreakVector (Transformation|GetActorLocation (Variables|/Game/Prototipagem/Mori/ControllerGame.ControllerGame_C|GetPlayer1 _returnvalue)))))) "Undefined" 0 0))
      (Variables|/Game/Prototipagem/Mori/AlvoItemJogado.AlvoItemJogado_C|SetPlayerAimed _returnvalue_2 (Variables|/Game/Prototipagem/Mori/ControllerGame.ControllerGame_C|GetPlayer1 _returnvalue))
      (switch int (Math|Random|RandomIntegerinRange 0 1)
        (:0
          (Default|SetasBuff _returnvalue_2))))
    (:2
      (bind _returnvalue_3 (Game|SpawnActorfromClass "/Game/Prototipagem/Mori/AlvoItemJogado.AlvoItemJogado_C" (Math|Conversions|ToTransform(Vector) (Math|Vector|MakeVector (.X (Math|Vector|BreakVector (Transformation|GetActorLocation (Variables|/Game/Prototipagem/Mori/ControllerGame.ControllerGame_C|GetPlayer2 _returnvalue)))) (+ (.Y (Math|Vector|BreakVector (Transformation|GetActorLocation (Variables|/Game/Prototipagem/Mori/ControllerGame.ControllerGame_C|GetPlayer2 _returnvalue)))) (Math|Random|RandomFloatinRange -3e+01 3e+01)) (.Z (Math|Vector|BreakVector (Transformation|GetActorLocation (Variables|/Game/Prototipagem/Mori/ControllerGame.ControllerGame_C|GetPlayer2 _returnvalue)))))) "Undefined" 0 0))
      (Variables|/Game/Prototipagem/Mori/AlvoItemJogado.AlvoItemJogado_C|SetPlayerAimed _returnvalue_3 (Variables|/Game/Prototipagem/Mori/ControllerGame.ControllerGame_C|GetPlayer2 _returnvalue))
      (switch int (Math|Random|RandomIntegerinRange 0 1)
        (:0
          (Default|SetasBuff _returnvalue_3))))))

(event EventBeginPlay
  (Utilities|FlowControl|Delay 6.0 :!label _label)
  (CallFunction|Fire)
  (goto _label))

(event Collision|EventActorBeginOverlap
  (params (OtherActor :type Actor%20Object%20Reference)))

(event EventTick
  (params (DeltaSeconds :type Float%20%28single-precision%29)))

(fn ConstructionScript)