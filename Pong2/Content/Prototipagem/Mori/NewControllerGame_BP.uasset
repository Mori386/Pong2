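; Game controller for a two-player ball game with parries, dashes and character ultimates, loading each player's chosen meshes and driving the HUD.
; A tick dispatcher applies physics-force movement to human players only.
; Ball hits grant energy; parried hits grant more and accelerate the ball.
; Energy pays for dashes and ultimates (clone balls, enlarged shield, invisible balls or zigzag balls), with a shared flag blocking overlapping ultimates.
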(event OnComponentHit(Player2)
  (params (HitComponent :type Primitive%20Component%20Object%20Reference) (OtherActor :type Actor%20Object%20Reference) (OtherComp :type Primitive%20Component%20Object%20Reference) (NormalImpulse :type Vector :default "0, 0, 0") (Hit :type Hit%20Result%20Structure%20%28by%20ref%29))
  (bind _player2 (Variables|Default|GetPlayer2))
  (bind _p2data (Variables|Default|GetP2Data))
  ;[1 0.3143 -0.0381] OnBallHit
  (bind _asbp_ball (Utilities|Casting|CastToBP_Ball OtherActor))
  (bind _doublehit (Default|IsComponentDoubleHit _asbp_ball _player2))
  (if (not _doublehit)
    (Default|HitonPlayer _asbp_ball _player2)
    (Development|PrintString "Hit")
    (if (Variables|/Game/Prototipagem/Mori/PlayerData.PlayerData_C|GetOnParry _p2data)
      (Utilities|FlowControl|Sequence
        (:then_0
          (if (Variables|/Game/Prototipagem/Mori/BP_Ball.BP_Ball_C|GetAccelerated _asbp_ball)
            _
            (else
              (Default|Accelerate _asbp_ball 1.0)))
          (CallFunction|ModifyEnergyOfPlayer 1e+01 _p2data)
          (CallFunction|ApplyEnergytoHUD _p2data :!label _label))
        (:then_1
          (Utilities|ParryHUDVisual _p2data)))
      (else
        (if (Variables|/Game/Prototipagem/Mori/BP_Ball.BP_Ball_C|GetAccelerated _asbp_ball)
          (Default|ResetAcceleration _asbp_ball))
        (CallFunction|ModifyEnergyOfPlayer 5.0 _p2data)
        (goto _label)))))

(event OnComponentHit(Player1)
  (params (HitComponent :type Primitive%20Component%20Object%20Reference) (OtherActor :type Actor%20Object%20Reference) (OtherComp :type Primitive%20Component%20Object%20Reference) (NormalImpulse :type Vector :default "0, 0, 0") (Hit :type Hit%20Result%20Structure%20%28by%20ref%29))
  (bind _p1data (Variables|Default|GetP1Data))
  (bind _player1 (Variables|Default|GetPlayer1))
  ;[1 0.3143 -0.0381] OnBallHit
  (bind _asbp_ball (Utilities|Casting|CastToBP_Ball OtherActor))
  (bind _doublehit (Default|IsComponentDoubleHit _asbp_ball _player1))
  (if (not _doublehit)
    (Default|HitonPlayer _asbp_ball _player1)
    (Development|PrintString "Hit")
    (if (Variables|/Game/Prototipagem/Mori/PlayerData.PlayerData_C|GetOnParry _p1data)
      (Utilities|FlowControl|Sequence
        (:then_0
          (if (Variables|/Game/Prototipagem/Mori/BP_Ball.BP_Ball_C|GetAccelerated _asbp_ball)
            _
            (else
              (Default|Accelerate _asbp_ball 1.0)))
          (CallFunction|ModifyEnergyOfPlayer 1e+01 _p1data)
          (CallFunction|ApplyEnergytoHUD _p1data :!label _label))
        (:then_1
          (Utilities|ParryHUDVisual _p1data)))
      (else
        (if (Variables|/Game/Prototipagem/Mori/BP_Ball.BP_Ball_C|GetAccelerated _asbp_ball)
          (Default|ResetAcceleration _asbp_ball))
        (CallFunction|ModifyEnergyOfPlayer 5.0 _p1data)
        (goto _label)))))

(event Custom|Player1ForceControl
  ;[1 1 -0.219 0.3905] Define player check input or ai controlled for movement control
  (CallFunction|ApplyForcetoPlayer (Variables|Default|GetPlayer1) (Variables|Default|GetP1Data) (Input|AxisValues|GetPlayer1VerticalControl) (Input|AxisValues|GetPlayer1HorizontalControl)))

(event Custom|Player2ForceControl
  ;[1 1 -0.219 0.3905] Define player check input or ai controlled for movement control
  (CallFunction|ApplyForcetoPlayer (Variables|Default|GetPlayer2) (Variables|Default|GetP2Data) (Input|AxisValues|GetPlayer2VerticalControl) (Input|AxisValues|GetPlayer2HorizontalControl)))

(event EventBeginPlay
  (Utilities|FlowControl|Sequence
    (:then_0
      ;[0.05714 1 1] HUD
      (bind _returnvalue (UserInterface|CreateWidget "/Game/Prototipagem/Mori/HUDIngame.HUDIngame_C"))
      (bind _output_get (Variables|Default|SetHUD _returnvalue))
      (UserInterface|Viewport|AddtoViewport _output_get 0))
    (:then_1
      ;[0.4449 0.1631 0.616] Set Original Balls
      (bind _outactors (Actor|GetAllActorsOfClass "/Game/Prototipagem/Mori/BP_Ball.BP_Ball_C"))
      (Variables|Default|SetOriginalBalls _outactors))
    (:then_2
      ;[1 1 -0.219 0.3905] Define player check input or ai controlled for movement control
      (if (Variables|/Game/Prototipagem/Mori/PlayerData.PlayerData_C|GetisAI (Variables|Default|GetP1Data))
        _
        (else
          (EventDispatchers|BindEventtoOnTickEvent (delegate Custom|Player1ForceControl))))
      (if (not (Variables|/Game/Prototipagem/Mori/PlayerData.PlayerData_C|GetisAI (Variables|Default|GetP2Data)))
        (EventDispatchers|BindEventtoOnTickEvent (delegate Custom|Player2ForceControl))))
    (:then_3
      ;[1 0.6432 0.6133] Mesh Personagens
      (Input|SetInputModeGameOnly (Game|GetPlayerController 0))
      (bind _asmy_game_instance (Utilities|Casting|CastToMyGameInstance (Game|GetGameInstance)))
      (Variables|/Game/Prototipagem/Mori/PlayerData.PlayerData_C|SetCharacterIndex (Variables|Default|GetP1Data) (Variables|/Game/Telas/TelaSeleção/MyGameInstance.MyGameInstance_C|GetCharacterindexPlayer1 _asmy_game_instance))
      (Variables|/Game/Prototipagem/Mori/PlayerData.PlayerData_C|SetCharacterIndex (Variables|Default|GetP2Data) (Variables|/Game/Telas/TelaSeleção/MyGameInstance.MyGameInstance_C|GetCharacterindexPlayer2 _asmy_game_instance)))
    (:then_4
      (CallFunction|LoadPlayersData))))

(event EventTick
  (params (DeltaSeconds :type Float%20%28single-precision%29))
  ;[1 1 -0.219 0.3905] Define player check input or ai controlled for movement control
  (Default|CallOnTickEvent))

(event Input|ActionEvents|InputActionP1Parry
  (params (Key :type Key%20Structure :default "None"))
  (bind _p1data (Variables|Default|GetP1Data))
  ;[1 0.2381 1] Parry
  (:Pressed
    (if (not (Variables|/Game/Prototipagem/Mori/PlayerData.PlayerData_C|GetisAI _p1data))
      (Utilities|Parry _p1data))))

(event Input|ActionEvents|InputActionP2Parry
  (params (Key :type Key%20Structure :default "None"))
  (bind _p2data (Variables|Default|GetP2Data))
  ;[1 0.2381 1] Parry
  (:Pressed
    (if (not (Variables|/Game/Prototipagem/Mori/PlayerData.PlayerData_C|GetisAI _p2data))
      (Utilities|Parry _p2data))))

(event Input|ActionEvents|InputActionP1Dash
  (params (Key :type Key%20Structure :default "None"))
  (bind _p1data (Variables|Default|GetP1Data))
  ;[0 1 0.4914] Dash
  (:Pressed
    (if (not (Variables|/Game/Prototipagem/Mori/PlayerData.PlayerData_C|GetisAI _p1data))
      (Utilities|Dash (Variables|Default|GetPlayer1) _p1data (Input|AxisValues|GetPlayer1HorizontalControl) (Input|AxisValues|GetPlayer1VerticalControl)))))

(event Input|ActionEvents|InputActionP2Dash
  (params (Key :type Key%20Structure :default "None"))
  (bind _p2data (Variables|Default|GetP2Data))
  ;[0 1 0.4914] Dash
  (:Pressed
    (if (not (Variables|/Game/Prototipagem/Mori/PlayerData.PlayerData_C|GetisAI _p2data))
      (Utilities|Dash (Variables|Default|GetPlayer2) _p2data (Input|AxisValues|GetPlayer2HorizontalControl) (Input|AxisValues|GetPlayer2VerticalControl)))))

(event Input|ActionEvents|InputActionP1Ult
  (params (Key :type Key%20Structure :default "None"))
  ;[1 0 0] Ultimate
  (:Pressed
    (if (not (Variables|Default|GetisUltimateGoingOn))
      (Utilities|Ultimate (Variables|Default|GetPlayer1) (Variables|Default|GetP1Data)))))

(event Input|ActionEvents|InputActionP2Ult
  (params (Key :type Key%20Structure :default "None"))
  ;[1 0 0] Ultimate
  (:Pressed
    (if (not (Variables|Default|GetisUltimateGoingOn))
      (Utilities|Ultimate (Variables|Default|GetPlayer2) (Variables|Default|GetP2Data)))))

(fn ConstructionScript)

(fn LoadPlayersData
  ;[1 0 0 0.3905] EnergySetup
  (CallFunction|ApplyEnergytoHUD (Variables|Default|GetP1Data))
  (CallFunction|ApplyEnergytoHUD (Variables|Default|GetP2Data))
  ;[0 1 0] HPSetup
  (CallFunction|ApplyHPtoHUD (Variables|Default|GetP1Data))
  (CallFunction|ApplyHPtoHUD (Variables|Default|GetP2Data))
  ;[1 0 0.1204] Load Meshes selecionadas
  (bind _mesh (Default|BasedonCharacterIndexReturnCharacterMesh (Variables|Default|GetP1Data)))
  (Class|SkinnedMeshComponent|SetSkeletalMesh (Variables|Default|GetPlayer1-Mesh) _mesh true)
  (bind _mesh_2 (Default|BasedonCharacterIndexReturnCharacterMesh (Variables|Default|GetP2Data)))
  (Class|SkinnedMeshComponent|SetSkeletalMesh (Variables|Default|GetPlayer2-Mesh) _mesh_2 true)
  ;[0.5987 0.03805 1] Load o escudo pré-definido
  (bind _material (Default|BasedonCharacterIndexReturnShieldMesh (Variables|Default|GetP1Data)))
  (Rendering|Material|SetMaterial (Variables|Default|GetPlayer1) 0 _material)
  (bind _material_2 (Default|BasedonCharacterIndexReturnShieldMesh (Variables|Default|GetP2Data)))
  (Rendering|Material|SetMaterial (Variables|Default|GetPlayer2) 0 _material_2))

(fn ApplyEnergytoHUD
  (params (PlayerData :type Player%20Data%20Object%20Reference))
  (bind _hud (Variables|Default|GetHUD))
  (bind _p2data (Variables|Default|GetP2Data))
  (bind _p1data (Variables|Default|GetP1Data))
  (bind _hud_2 (Variables|Default|GetHUD))
  (bind _energy (Variables|/Game/Prototipagem/Mori/PlayerData.PlayerData_C|GetEnergy _p2data))
  (bind _energy_2 (Variables|/Game/Prototipagem/Mori/PlayerData.PlayerData_C|GetEnergy _p1data))
  (if (== (Variables|Default|GetP1Data) PlayerData)
    (Rendering|Components|TextRender|SetText (Variables|/Game/Prototipagem/Mori/HUDIngame.HUDIngame_C|GetP1EnergyAmount _hud_2) (Utilities|Text|ToText(Float) _energy_2 "HalfToEven"))
    (Progress|SetPercent (Variables|/Game/Prototipagem/Mori/HUDIngame.HUDIngame_C|GetP1EnergyBar _hud_2) (/ _energy_2 (Variables|/Game/Prototipagem/Mori/PlayerData.PlayerData_C|GetEnergyMax _p1data)))
    (else
      (Rendering|Components|TextRender|SetText (Variables|/Game/Prototipagem/Mori/HUDIngame.HUDIngame_C|GetP2EnergyAmount _hud) (Utilities|Text|ToText(Float) _energy "HalfToEven"))
      (Progress|SetPercent (Variables|/Game/Prototipagem/Mori/HUDIngame.HUDIngame_C|GetP2EnergyBar _hud) (/ _energy (Variables|/Game/Prototipagem/Mori/PlayerData.PlayerData_C|GetEnergyMax _p2data))))))

(fn ApplyHPtoHUD
  (params (PlayerData :type Player%20Data%20Object%20Reference))
  (bind _p1data (Variables|Default|GetP1Data))
  (bind _hud (Variables|Default|GetHUD))
  (bind _p2data (Variables|Default|GetP2Data))
  (bind _hud_2 (Variables|Default|GetHUD))
  (bind _hp (Variables|/Game/Prototipagem/Mori/PlayerData.PlayerData_C|GetHP _p2data))
  (bind _hp_2 (Variables|/Game/Prototipagem/Mori/PlayerData.PlayerData_C|GetHP _p1data))
  (if (== PlayerData (Variables|Default|GetP1Data))
    (Rendering|Components|TextRender|SetText (Variables|/Game/Prototipagem/Mori/HUDIngame.HUDIngame_C|GetP1HPAmount _hud) (Utilities|Text|ToText(Integer) _hp_2))
    (Progress|SetPercent (Variables|/Game/Prototipagem/Mori/HUDIngame.HUDIngame_C|GetP1HPBar _hud) (/ (Math|Conversions|ToFloat(Integer) _hp_2) (Math|Conversions|ToFloat(Integer) (Variables|/Game/Prototipagem/Mori/PlayerData.PlayerData_C|GetHPMax _p1data))))
    (else
      (Rendering|Components|TextRender|SetText (Variables|/Game/Prototipagem/Mori/HUDIngame.HUDIngame_C|GetP2HPAmount _hud_2) (Utilities|Text|ToText(Integer) _hp))
      (Progress|SetPercent (Variables|/Game/Prototipagem/Mori/HUDIngame.HUDIngame_C|GetP2HPBar _hud_2) (/ (Math|Conversions|ToFloat(Integer) _hp) (Math|Conversions|ToFloat(Integer) (Variables|/Game/Prototipagem/Mori/PlayerData.PlayerData_C|GetHPMax _p2data)))))))

(fn ApplyForcetoPlayer
  (params (Player :type Static%20Mesh%20Component%20Object%20Reference) (PlayerData :type Player%20Data%20Object%20Reference) (PlayerInputAxisVertical :type Float%20%28single-precision%29) (PlayerInputAxisHorizontal :type Float%20%28single-precision%29))
  (if (== PlayerInputAxisVertical 0.0)
    (if (not (== PlayerInputAxisHorizontal 0.0))
      (bind _returnvalue (Physics|GetPhysicsLinearVelocity Player "None" :!label _label))
      (if (not (> (+ (Math|Float|Absolute(Float) (.X (Math|Vector|BreakVector _returnvalue))) (Math|Float|Absolute(Float) (.Y (Math|Vector|BreakVector _returnvalue)))) (Variables|/Game/Prototipagem/Mori/PlayerData.PlayerData_C|GetMaxSpeed PlayerData)))
        (Physics|AddForce Player (* (Math|Vector|MakeVector PlayerInputAxisHorizontal PlayerInputAxisVertical 0.0) (* (Variables|/Game/Prototipagem/Mori/PlayerData.PlayerData_C|GetAcceleration PlayerData) 2e+02)) "None" false)))
    (else
      (goto _label))))

(fn ModifyEnergyOfPlayer
  (params (Energy :type Float%20%28single-precision%29) (PlayerData :type Player%20Data%20Object%20Reference))
  (bind _energymax (Variables|/Game/Prototipagem/Mori/PlayerData.PlayerData_C|GetEnergyMax PlayerData))
  (if (>= (+ Energy (Variables|/Game/Prototipagem/Mori/PlayerData.PlayerData_C|GetEnergy PlayerData)) 0.0)
    (if (> (+ Energy (Variables|/Game/Prototipagem/Mori/PlayerData.PlayerData_C|GetEnergy PlayerData)) _energymax)
      (Variables|/Game/Prototipagem/Mori/PlayerData.PlayerData_C|SetEnergy PlayerData _energymax)
      (else
        (Variables|/Game/Prototipagem/Mori/PlayerData.PlayerData_C|SetEnergy PlayerData (+ Energy (Variables|/Game/Prototipagem/Mori/PlayerData.PlayerData_C|GetEnergy PlayerData)))))))

(fn ModifyHPOfPlayer
  (params (PlayerData :type Player%20Data%20Object%20Reference) (HP :type Integer))
  (if (> (+ (Variables|/Game/Prototipagem/Mori/PlayerData.PlayerData_C|GetHP PlayerData) HP) 0)
    (if (<= (+ (Variables|/Game/Prototipagem/Mori/PlayerData.PlayerData_C|GetHP PlayerData) HP) (Variables|/Game/Prototipagem/Mori/PlayerData.PlayerData_C|GetHPMax PlayerData))
      (Variables|/Game/Prototipagem/Mori/PlayerData.PlayerData_C|SetHP PlayerData (+ (Variables|/Game/Prototipagem/Mori/PlayerData.PlayerData_C|GetHP PlayerData) HP)))))

(fn CheckBallDoubleHitList
  (params (Bal :type BP%20Ball%20Object%20Reference) (PlayerData :type Player%20Data%20Object%20Reference))
  (bind _array_element (Utilities|Array|ForEachLoopwithBreak (Variables|/Game/Prototipagem/Mori/PlayerData.PlayerData_C|GetDoubleHitBallsList PlayerData) :!label _label)
    (:LoopBody
      (if (== _array_element Bal)
        (LocalVariables|SetDoubleHitted true)
        (goto _label Break)))
    (:Completed
      (return (LocalVariables|GetDoubleHitted)))))

(fn GetPlayerIndexfromData
  (params (PlayerData :type Player%20Data%20Object%20Reference))
  (bind _array_element (Utilities|Array|ForEachLoopwithBreak (Utilities|String|GetCharacterArrayfromString (Utilities|GetObjectName PlayerData)) :!label _label)
    (:LoopBody
      (if (Class|KismetStringLibrary|IsNumeric _array_element)
        (Utilities|FlowControl|Sequence
          (:then_0
            (goto _label Break))
          (:then_1
            (return (Math|Conversions|ToInteger(Byte) _array_element))))))
    (:Completed
      (return -1))))